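; Big loot crate that the player opens with E while inside its interact box, with input and a gate toggled by overlap.
; Opening plays timelines for the lid and two side displays plus a sound, then spawns a rifle and two randomly chosen addon pickups.
; Delays later destroy the spawns, reverse the timelines and reset the crate for reuse.
; The weapon roll always yields the rifle, as the pistol spawn is unconnected.
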(event `self.ReceiveBeginPlay`
  (`|ExecutionSequence`
    (:`then_0`
      (set `self.Opened` false))))

(event `Key|E`
  (params (Key :type "Key Structure"))
  (:`Pressed`
    (if (and (`self.Player Close`) (not (`self.Opened`)))
      (`/Engine/EditorBlueprintResources/StandardMacros.Gate` true :!label _label
        (:`Exit`
          (set `self.Opened` true)
          (`|ExecutionSequence`
            (:`then_0`
              (`|ExecutionSequence`
                (:`then_0`
                  (`KismetSystemLibrary.Delay` 29.5)
                  (set `self.Opened` false)
                  (bind (_direction _open__pitch_) (`Timeline|Open Big Crate Timeline` :!via `Reverse` :!label _label_2)
                    (:`Update`
                      (`SceneComponent.K2_SetRelativeRotation` (`self.PivotTop`) (`KismetMathLibrary.MakeRotator` 0.0 _open__pitch_) false false))))
                (:`then_1`
                  (goto _label_2))
                (:`then_2`
                  (`GameplayStatics.PlaySoundAtLocation` "/Game/Audio/Effects/Chests/BigChest_Audio.BigChest_Audio" (`SceneComponent.K2_GetComponentLocation` (`self.BigCrate2 (Outline)`)) (struct) 1.0 1.0 0.0 null null null null))))
            (:`then_1`
              (`|ExecutionSequence`
                (:`then_0`
                  (`KismetSystemLibrary.Delay` 29.0)
                  (bind (_direction_2 _display_1__roll_) (`Timeline|Big Crate Display 1 Timeline` :!via `Reverse` :!label _label_3)
                    (:`Update`
                      (`SceneComponent.K2_SetRelativeRotation` (`self.PivotDisplay1`) (`KismetMathLibrary.MakeRotator` _display_1__roll_) false false))))
                (:`then_1`
                  (goto _label_3))))
            (:`then_2`
              (`|ExecutionSequence`
                (:`then_0`
                  (`KismetSystemLibrary.Delay` 29.0)
                  (bind (_direction_3 _display_2__roll_) (`Timeline|Big Crate Display 2 Timeline` :!via `Reverse` :!label _label_4)
                    (:`Update`
                      (`SceneComponent.K2_SetRelativeRotation` (`self.PivotDisplay2`) (`KismetMathLibrary.MakeRotator` _display_2__roll_) false false))))
                (:`then_1`
                  (goto _label_4))))
            (:`then_4`
              (`self.Random Weapon spawner`))
            (:`then_5`
              (`self.Random Addon Spawner`)))))
      (else
        (`KismetSystemLibrary.PrintText` "Already Open")))))

(event `self.InteractBox.OnComponentBeginOverlap`
  (params (OverlappedComponent :type "PrimitiveComponent Object Reference") (OtherActor :type "Actor Object Reference") (OtherComp :type "PrimitiveComponent Object Reference") (OtherBodyIndex :type Integer) (bFromSweep :type Boolean) (SweepResult :type "HitResult Structure (by ref)"))
  (bind _asbp_first_person_character (cast `/Game/FirstPerson/Blueprints/BP_FirstPersonCharacter` OtherActor))
  (set `self.Player` _asbp_first_person_character)
  (`self.EnableInput` (`GameplayStatics.GetPlayerController` 0))
  (`|ExecutionSequence`
    (:`then_0`
      (goto _label :!via `Open`))
    (:`then_1`
      (set `self.Player Close` true))))

(event `self.InteractBox.OnComponentEndOverlap`
  (params (OverlappedComponent :type "PrimitiveComponent Object Reference") (OtherActor :type "Actor Object Reference") (OtherComp :type "PrimitiveComponent Object Reference") (OtherBodyIndex :type Integer))
  (bind _asbp_first_person_character (cast `/Game/FirstPerson/Blueprints/BP_FirstPersonCharacter` OtherActor))
  (set `self.Player` _asbp_first_person_character)
  (`self.DisableInput` (`GameplayStatics.GetPlayerController` 0))
  (`|ExecutionSequence`
    (:`then_0`
      (goto _label :!via `Close`))
    (:`then_1`
      (set `self.Player Close` false))))

(event `Random Weapon spawner`
  (bind _weaponspawnpoint (`self.WeaponSpawnPoint`))
  (`|ExecutionSequence`
    (:`then_0`
      (`KismetSystemLibrary.Delay` 29.0)
      (`self.K2_DestroyActor` (stale _returnvalue)))
    (:`then_1`
      (`KismetSystemLibrary.Delay` 0.3)
      (bind _output_get (set `self.Weapon Spawn` (`KismetMathLibrary.RandomIntegerInRange` 1 2)))
      (if (== _output_get 1)
        _
        (else
          _))
      (bind _returnvalue (`|SpawnActorFromClass` "/Game/Weapons/BP_Weapons/BP_Rifle.BP_Rifle_C" (`KismetMathLibrary.MakeTransform` (`SceneComponent.K2_GetComponentLocation` _weaponspawnpoint) (`SceneComponent.K2_GetComponentRotation` _weaponspawnpoint) (`SceneComponent.K2_GetComponentScale` _weaponspawnpoint)) "Undefined" "OverrideRootScale" null 15 3 null)))))

(event `Random Addon Spawner`
  (bind _addonspawner2 (`self.AddonSpawner2`))
  (bind _addonspawner1 (`self.AddonSpawner1`))
  (bind _returnvalue (`KismetMathLibrary.MakeTransform` (`SceneComponent.K2_GetComponentLocation` _addonspawner2) (`SceneComponent.K2_GetComponentRotation` _addonspawner2) (`SceneComponent.K2_GetComponentScale` _addonspawner2)))
  (bind _returnvalue_2 (`KismetMathLibrary.MakeTransform` (`SceneComponent.K2_GetComponentLocation` _addonspawner1) (`SceneComponent.K2_GetComponentRotation` _addonspawner1) (`SceneComponent.K2_GetComponentScale` _addonspawner1)))
  (`|ExecutionSequence`
    (:`then_0`
      (`KismetSystemLibrary.Delay` 29.0)
      (`self.K2_DestroyActor` (stale _returnvalue_3))
      (`self.K2_DestroyActor` (stale _returnvalue_4))
      (`self.K2_DestroyActor` (stale _returnvalue_5))
      (`self.K2_DestroyActor` (stale _returnvalue_6))
      (`self.K2_DestroyActor` (stale _returnvalue_7)))
    (:`then_1`
      (`KismetSystemLibrary.Delay` 0.75)
      (`|ExecutionSequence`
        (:`then_0`
          (bind _output_get (set `self.Addon Spawn1` (`KismetMathLibrary.RandomIntegerInRange` 1 2)))
          (if (== _output_get 1)
            (bind _returnvalue_3 (`|SpawnActorFromClass` "/Game/Pickups/Powerups/KevlarPickup_BP.KevlarPickup_BP_C" _returnvalue_2 "Undefined" "OverrideRootScale" null null))
            (else
              (bind _returnvalue_4 (`|SpawnActorFromClass` "/Game/Pickups/Powerups/BootPickup_BP.BootPickup_BP_C" _returnvalue_2 "Undefined" "OverrideRootScale" null null)))))
        (:`then_1`
          (bind _output_get_2 (set `self.Addon Spawn2` (`KismetMathLibrary.RandomIntegerInRange` 1 3)))
          (if (== _output_get_2 1)
            (bind _returnvalue_5 (`|SpawnActorFromClass` "/Game/Pickups/Powerups/HelmetPickup_BP.HelmetPickup_BP_C" _returnvalue "Undefined" "OverrideRootScale" null null))
            (elif (== _output_get_2 2)
              (bind _returnvalue_6 (`|SpawnActorFromClass` "/Game/Pickups/Powerups/NormalMag_BP.NormalMag_BP_C" _returnvalue "Undefined" "OverrideRootScale" null null))
              (else
                (bind _returnvalue_7 (`|SpawnActorFromClass` "/Game/Pickups/Powerups/SpecialMag_BP.SpecialMag_BP_C" _returnvalue "Undefined" "OverrideRootScale" null null))))))))))

(fn `UserConstructionScript`)