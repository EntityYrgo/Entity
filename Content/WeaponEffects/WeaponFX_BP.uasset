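; Weapon effects Blueprint that plays a Niagara muzzle flash when its weapon fires.
; WeaponFire reuses one attached Niagara component, spawning a new one at the root using the muzzle socket's location only when it is invalid or inactive.
; Each shot passes the normalized muzzle-to-first-impact direction and flips a Boolean trigger parameter to signal the system, rather than respawning it.
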(event `WeaponFire`
  (params (Hit :type "HitResult Structure"))
  (bind _muzzleflash_ns (`self.MuzzleFlash_NS`))
  (bind _returnvalue (`SceneComponent.GetSocketLocation` (`self.WeaponMesh`) (`self.MuzzleSocket`)))
  (`|ExecutionSequence`
    (:`then_0`
      (`/Engine/EditorBlueprintResources/StandardMacros.IsValid` (`self.MuzzleFlash_NS`)
        (:`Is Valid`
          (if (not (`ActorComponent.IsActive` (`self.MuzzleFlash_NS`)))
            (bind _returnvalue_2 (`NiagaraFunctionLibrary.SpawnSystemAttached` (`self.MuzzleFlash_FX`) (`self.DefaultSceneRoot`) "None" _returnvalue (struct) "KeepRelativeOffset" :!label _label))
            (set `self.MuzzleFlash_NS` _returnvalue_2)
            (set `self.MuzzleFlashTrigger` false)))
        (:`Is Not Valid`
          (goto _label)))
      (set `self.MuzzleFlashTrigger` (not (`self.MuzzleFlashTrigger`)))
      (`NiagaraComponent.SetVariableVec3` _muzzleflash_ns "User.Direction" (`KismetMathLibrary.Normal` (- (`|GetArrayItem` (`self.Impact Positions`)) _returnvalue)))
      (`NiagaraComponent.SetVariableBool` _muzzleflash_ns "User.Trigger" (`self.MuzzleFlashTrigger`)))))

(fn `UserConstructionScript`)