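; AL-37 rifle magazine pickup that the first-person character collects by pressing E while inside its trigger box.
; Box overlap toggles input and a gate, and clears the player's pickup text on exit.
; On E, it finds the rifle via GetActorOfClass and, if the player has a rifle but no mag attached, adds ammo to rifle and player, flags the mag attached, plays a sound and destroys itself.
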(event `self.ReceiveBeginPlay`
  (`|ExecutionSequence`
    (:`then_0`
      (set `self.Name` "AL-37 Mag"))))

(event `Key|E`
  (params (Key :type "Key Structure"))
  (bind _rifle_ref (`self.Rifle REF`))
  (bind _player (`self.Player`))
  (bind _player_2 (`self.Player`))
  (bind _player_3 (`self.Player`))
  (:`Pressed`
    (if (`self.PlayerOverlap`)
      (`/Engine/EditorBlueprintResources/StandardMacros.Gate` true :!label _label
        (:`Exit`
          (bind _returnvalue (`GameplayStatics.GetActorOfClass` "/Game/Weapons/BP_Weapons/BP_Rifle.BP_Rifle_C"))
          (set `self.Rifle REF` _returnvalue)
          (if (and (not (`/Game/FirstPerson/Blueprints/BP_FirstPersonCharacter.RifleMagAttached` _player_2)) (`/Game/FirstPerson/Blueprints/BP_FirstPersonCharacter.RifleAttached` _player_2))
            (`|ExecutionSequence`
              (:`then_0`
                (set `/Game/Weapons/BP_Weapons/BP_Rifle.MaxRifleAmmo` (+ (`/Game/Weapons/BP_Weapons/BP_Rifle.MaxRifleAmmo` _rifle_ref) (`self.RifleMag`)) _rifle_ref)
                (set `/Game/FirstPerson/Blueprints/BP_FirstPersonCharacter.RifleMagAttached` true _player)
                (`GameplayStatics.PlaySoundAtLocation` "/Game/SoundEffects/MagPickup.MagPickup" (`SceneComponent.K2_GetComponentLocation` (`/Game/FirstPerson/Blueprints/BP_FirstPersonCharacter.LegBox` _player)) (struct) 1.0 1.0 0.0 null null null null)
                (`self.K2_DestroyActor`))
              (:`then_1`
                (set `/Game/FirstPerson/Blueprints/BP_FirstPersonCharacter.MaxRifleAmmo` (+ (`/Game/FirstPerson/Blueprints/BP_FirstPersonCharacter.MaxRifleAmmo` _player_3) (`self.RifleMag`)) _player_3)))))))))

(event `self.Box.OnComponentBeginOverlap`
  (params (OverlappedComponent :type "PrimitiveComponent Object Reference") (OtherActor :type "Actor Object Reference") (OtherComp :type "PrimitiveComponent Object Reference") (OtherBodyIndex :type Integer) (bFromSweep :type Boolean) (SweepResult :type "HitResult Structure (by ref)"))
  (bind _asbp_first_person_character (cast `/Game/FirstPerson/Blueprints/BP_FirstPersonCharacter` OtherActor))
  (set `self.Player` _asbp_first_person_character)
  (`self.EnableInput` (`GameplayStatics.GetPlayerController` 0))
  (`|ExecutionSequence`
    (:`then_0`
      (goto _label :!via `Open`))
    (:`then_1`
      (set `self.PlayerOverlap` true))))

(event `self.Box.OnComponentEndOverlap`
  (params (OverlappedComponent :type "PrimitiveComponent Object Reference") (OtherActor :type "Actor Object Reference") (OtherComp :type "PrimitiveComponent Object Reference") (OtherBodyIndex :type Integer))
  (bind _asbp_first_person_character (cast `/Game/FirstPerson/Blueprints/BP_FirstPersonCharacter` OtherActor))
  (set `self.Player` _asbp_first_person_character)
  (`self.DisableInput` (`GameplayStatics.GetPlayerController` 0))
  (`|ExecutionSequence`
    (:`then_0`
      (goto _label :!via `Close`))
    (:`then_1`
      (set `self.PlayerOverlap` false))
    (:`then_2`
      (`/Game/WidgetBlueprints/WB_PickupText.SetText` (`/Game/FirstPerson/Blueprints/BP_FirstPersonCharacter.PickUpText_Ref` (`self.Player`)) ""))))

(fn `GetDurability/ammo`
  (returns (`Durability/ammo` :type Integer)))

(fn `GetName`
  (returns (Name :type Text))
  (return (`self.Name`)))

(fn `UserConstructionScript`)