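; AL-37 Assault rifle pickup actor that reports its name, pickup type and ammo counts through getters.
; On BeginPlay it initializes ammo, and the server spawns and attaches a hidden BP_ChildRifle.
; TextCollision overlaps toggle the first-person character's pickup state, while custom depth stencil drives the outline.
; A dynamic material switches the lamp's emissive strength, and BreakEffect hides the rifle parts and activates Niagara.
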(event `EnableOutline`
  (`PrimitiveComponent.SetCustomDepthStencilValue` (`self.Static Mesh`) 2))

(event `DisableOutline`
  (`PrimitiveComponent.SetCustomDepthStencilValue` (`self.Static Mesh`) 0))

(event `self.ReceiveBeginPlay`
  ;[0 0 0] Event BeginPlay
  (`|ExecutionSequence`
    (:`then_0`
      (set `self.Name` "AL-37 Assault"))
    (:`then_1`
      (set `self.RifleAmmo` 25)
      (set `self.MaxRifleAmmo` 25))
    (:`then_2`
      (if (`KismetSystemLibrary.IsServer`)
        (`self.SpawnChildGun`)))
    (:`then_3`
      (`self.DisableOutline`))))

(event `SpawnChildGun`
  (bind _returnvalue (`|SpawnActorFromClass` "/Game/Weapons/BP_Weapons/BP_ChildRifle.BP_ChildRifle_C" (`self.GetTransform` self) "AlwaysSpawn" "OverrideRootScale" null null))
  (`SceneComponent.SetVisibility` (`/Game/Weapons/BP_Weapons/BP_ChildRifle.Static Mesh` _returnvalue) false true)
  (`self.K2_AttachToActor` _returnvalue self "None" "SnapToTarget" "SnapToTarget" "SnapToTarget" true))

(event `self.TextCollision.OnComponentBeginOverlap`
  (params (OverlappedComponent :type "PrimitiveComponent Object Reference") (OtherActor :type "Actor Object Reference") (OtherComp :type "PrimitiveComponent Object Reference") (OtherBodyIndex :type Integer) (bFromSweep :type Boolean) (SweepResult :type "HitResult Structure (by ref)"))
  ;[0 0 0] Checks if you can pick up pistol
  (bind _asbp_first_person_character (cast `/Game/FirstPerson/Blueprints/BP_FirstPersonCharacter` OtherActor))
  (set `/Game/FirstPerson/Blueprints/BP_FirstPersonCharacter.PickUpOverlapping` true _asbp_first_person_character))

(event `LampOn/Off`
  (params (`On/Off` :type Boolean))
  (bind _material (`self.Material`))
  (if `On/Off`
    (`MaterialInstanceDynamic.SetScalarParameterValue` _material "EmissiveMultiply" 500.0)
    (else
      (`MaterialInstanceDynamic.SetScalarParameterValue` _material "EmissiveMultiply" 50.0)))
  (`PrimitiveComponent.SetMaterial` (`self.Static Mesh`) 0 (`self.Material`)))

(event `self.TextCollision.OnComponentEndOverlap`
  (params (OverlappedComponent :type "PrimitiveComponent Object Reference") (OtherActor :type "Actor Object Reference") (OtherComp :type "PrimitiveComponent Object Reference") (OtherBodyIndex :type Integer))
  ;[0 0 0] Checks if you can pick up pistol
  (bind _asbp_first_person_character (cast `/Game/FirstPerson/Blueprints/BP_FirstPersonCharacter` OtherActor))
  (set `/Game/FirstPerson/Blueprints/BP_FirstPersonCharacter.PickUpOverlapping` false _asbp_first_person_character)
  (`/Game/WidgetBlueprints/WB_PickupText.SetText` (`/Game/FirstPerson/Blueprints/BP_FirstPersonCharacter.PickUpText_Ref` _asbp_first_person_character) ""))

(event `BreakEffect`
  (`SceneComponent.SetVisibility` (`self.Static Mesh`) false false)
  (`SceneComponent.SetVisibility` (`self.Trigger`) false false)
  (`SceneComponent.SetVisibility` (`self.HoloSight`) false false)
  (`ActorComponent.Activate` (`self.Niagara`) true))

(fn `GetDurability/ammo`
  (returns (`Durability/ammo` :type Integer))
  (return (`self.RifleAmmo`)))

(fn `GetName`
  (returns (Name :type Text))
  (return (`self.Name`)))

(fn `GetPickupType`
  (returns (Pickup :type "/Game/Pickups/EPickups Enum"))
  (return "NewEnumerator8"))

(fn `GetTotalAmmo`
  (returns (TotalAmmo :type Integer))
  (return (`self.MaxRifleAmmo`)))

(fn `GetTracerAmmo`
  (returns (TracerAmmo :type Integer))
  (return (`self.TracerAmmo`)))

(fn `UserConstructionScript`
  (bind _returnvalue (`KismetMaterialLibrary.CreateDynamicMaterialInstance` "/Game/Weapons/WeaponsMaterials/AL_37_ASSAULT_MAT.AL_37_ASSAULT_MAT"))
  (bind _output_get (set `self.Material` _returnvalue))
  (`MaterialInstanceDynamic.SetScalarParameterValue` _output_get "EmissiveMultiply" 500.0)
  (`PrimitiveComponent.SetMaterial` (`self.Static Mesh`) 0 (`self.Material`)))