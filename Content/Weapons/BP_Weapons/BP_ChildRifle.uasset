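; Rifle weapon Blueprint that handles a swappable holographic sight and a break effect.
; The holo sight starts hidden, and ChangeSight either hides it or shows it with an aim or infrared material on the crosshair display, based on a sight enum.
; BreakEffect hides the rifle mesh and sight component, then activates a Niagara effect.
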(event `BreakEffect`
  (`SceneComponent.SetVisibility` (`self.Static Mesh`) false false)
  (`SceneComponent.SetVisibility` (`self.HoloSight`) false false)
  (`ActorComponent.Activate` (`self.Niagara`) true))

(event `self.ReceiveBeginPlay`
  (`SceneComponent.SetVisibility` (`self.HoloSight`) false true))

(event `ChangeSight`
  (params (sight :type Byte :default 0))
  (if (not (`SceneComponent.IsVisible` (`self.HoloSight`)))
    (`SceneComponent.SetVisibility` (`self.HoloSight`) true true))
  (switch `|SwitchEnum` sight
    (:`NewEnumerator0`
      (`SceneComponent.SetVisibility` (`self.HoloSight`) false true))
    (:`NewEnumerator1`
      (`PrimitiveComponent.SetMaterial` (`self.HolographicSight_CrosshairDisplay`) 0 (`self.aimMat`)))
    (:`NewEnumerator2`
      (`PrimitiveComponent.SetMaterial` (`self.HolographicSight_CrosshairDisplay`) 0 (`self.infraredMat`)))))

(fn `UserConstructionScript`)