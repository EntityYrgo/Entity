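; BP_Pistol is a pistol pickup that shows a prompt when a character enters its collision.
; On BeginPlay it creates a hidden pickup widget, and only the server spawns a BP_ChildPistol with an invisible mesh attached to itself.
; Overlap events track PistolOverlap and toggle the prompt, which stays hidden if the character already has a pistol attached.
; The pickup action itself is not handled here.
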(event `SpawnChildGun`
  (bind _returnvalue (`|SpawnActorFromClass` "/Game/Weapons/BP_Weapons/BP_ChildPistol.BP_ChildPistol_C" (`self.GetTransform` self) "AlwaysSpawn" "OverrideRootScale" null null))
  (`SceneComponent.SetVisibility` (`/Game/Weapons/BP_Weapons/BP_ChildPistol.StaticMesh` _returnvalue) false true)
  (`self.K2_AttachToActor` _returnvalue self "None" "SnapToTarget" "SnapToTarget" "SnapToTarget" true))

(event `self.ReceiveBeginPlay`
  ;[0 0 0] Event BeginPlay
  (bind _returnvalue (`|CreateWidget` "/Game/JennysTest/WB_PickupText.WB_PickupText_C"))
  (`UserWidget.AddToViewport` _returnvalue 0)
  (bind _output_get (set `self.PickUp Widget` _returnvalue))
  (`Widget.SetVisibility` _output_get "Hidden")
  (if (`KismetSystemLibrary.IsServer`)
    (`self.SpawnChildGun`)))

(event `self.PickUpCollision.OnComponentBeginOverlap`
  (params (OverlappedComponent :type "PrimitiveComponent Object Reference") (OtherActor :type "Actor Object Reference") (OtherComp :type "PrimitiveComponent Object Reference") (OtherBodyIndex :type Integer) (bFromSweep :type Boolean) (SweepResult :type "HitResult Structure (by ref)"))
  ;[0 0 0] Checks if you can pick up pistol
  (set `self.PistolOverlap` true)
  (bind _asbp_third_person_character (cast `/Game/ThirdPerson/Blueprints/BP_ThirdPersonCharacter` OtherActor))
  (if (`/Game/ThirdPerson/Blueprints/BP_ThirdPersonCharacter.PistolAttached` _asbp_third_person_character)
    (`Widget.SetVisibility` (`self.PickUp Widget`) "Hidden")
    (else
      (`Widget.SetVisibility` (`self.PickUp Widget`) "Visible"))))

(event `self.PickUpCollision.OnComponentEndOverlap`
  (params (OverlappedComponent :type "PrimitiveComponent Object Reference") (OtherActor :type "Actor Object Reference") (OtherComp :type "PrimitiveComponent Object Reference") (OtherBodyIndex :type Integer))
  ;[0 0 0] Checks if you can pick up pistol
  (set `self.PistolOverlap` false)
  (`Widget.SetVisibility` (`self.PickUp Widget`) "Hidden"))

(fn `NewFunction`
  (`WidgetLayoutLibrary.RemoveAllWidgets`))

(fn `UserConstructionScript`)