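; Player controller for a networked shooter with session kick handling, a timer and a Tab-held leaderboard.
; The local controller requests a spawn, which the game mode performs through a server event.
; Shoot spawns a projectile tagged with the shooter's player state for attribution and plays the fire sound.
; EndGame forwards to the game state, while kicking opens the session menu and destroys the session.
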(event `StartSpawn`
  ;[1 0.4275 0.1608 0.3176] Spawn Player at Random PlayerStart
  (if (`self.IsLocalPlayerController`)
    (`self.Server_SpawnPlayer`)))

(event `Server_SpawnPlayer`
  ;[1 0.4275 0.1608 0.3176] Spawn Player at Random PlayerStart
  (bind _asmy_game_mode_bp (cast `/Game/Network_BP/MyGameMode_BP` (`GameplayStatics.GetGameMode`)))
  (`/Game/Network_BP/MyGameMode_BP.SpawnPlayer` _asmy_game_mode_bp self))

(event `AddGameWidgets`
  ;[1 0.4275 0.1608 0.3176] Add Leaderboard Widget
  (bind _returnvalue (`|CreateWidget` "/Game/Network_BP/Widgets/LeaderBoard_WB.LeaderBoard_WB_C" self))
  (bind _output_get (set `self.Leaderboard_Ref` _returnvalue))
  (`Widget.SetVisibility` _output_get "Collapsed")
  (`Widget.SetVisibility` (`/Game/Network_BP/Widgets/LeaderBoard_WB.ButtonBox` (`self.Leaderboard_Ref`)) "Collapsed")
  (`/Engine/EditorBlueprintResources/StandardMacros.IsValid` _output_get
    (:`Is Valid`
      (`UserWidget.AddToViewport` _output_get 0)
      ;[1 0.4275 0.1608 0.3176] Add timer widget
      (bind _returnvalue_2 (`|CreateWidget` "/Game/Network_BP/Widgets/Timer_WB.Timer_WB_C" self))
      (`/Engine/EditorBlueprintResources/StandardMacros.IsValid` _returnvalue_2
        (:`Is Valid`
          (`UserWidget.AddToViewport` _returnvalue_2 0))))))

(event `Shoot`
  (params (SpawnPos :type "Transform Structure") (Location :type "Vector Structure") (Weapon :type "Actor Object Reference"))
  (bind _playerstate (`self.PlayerState`))
  ;[1 0.2285 0.2584] Shoot
  (bind _returnvalue (`|SpawnActorFromClass` "/Game/FirstPerson/Blueprints/BP_FirstPersonProjectile.BP_FirstPersonProjectile_C" (`KismetMathLibrary.MakeTransform` SpawnPos_Location SpawnPos_Rotation) "AlwaysSpawn" "OverrideRootScale" (`PlayerState.GetPawn` _playerstate) null))
  (bind _asmy_player_state_bp (cast `/Game/Network_BP/MyPlayerState_BP` _playerstate))
  (set `/Game/FirstPerson/Blueprints/BP_FirstPersonProjectile.OwningPlayerstate` _asmy_player_state_bp _returnvalue)
  (`GameplayStatics.PlaySoundAtLocation` "/Game/FPWeapon/Audio/FirstPersonTemplateWeaponFire02.FirstPersonTemplateWeaponFire02" Location (struct) 1.0 1.0 0.0 null null null null))

(event `Key|P`
  (params (Key :type "Key Structure")))

(event `Key|Tab`
  (params (Key :type "Key Structure"))
  ;[1 0.5257 0.8814] Show/Hide Leaderboard
  (:`Pressed`
    (`Widget.SetVisibility` (`self.Leaderboard_Ref`) "Visible"))
  (:`Released`
    (`Widget.SetVisibility` (`self.Leaderboard_Ref`) "Collapsed")))

(event `EndGame`
  ;[0.3429 0.03419 0.3438] EndGame
  (bind _asmy_game_state_bp (cast `/Game/Network_BP/MyGameState_BP` (`GameplayStatics.GetGameState`)))
  (`/Game/Network_BP/MyGameState_BP.EndGame` _asmy_game_state_bp))

(event `OC_KickPlayer`
  (`GameplayStatics.OpenLevelBySoftObjectPtr` "/Game/Maps/SessionMenu.SessionMenu")
  (`DestroySessionCallbackProxy.DestroySession` null
    (:`OnSuccess`
      (`KismetSystemLibrary.PrintString` "Got kicked"))))

(fn `ClientTriggerAction`
  (bind _asmy_game_state_bp (cast `/Game/Network_BP/MyGameState_BP` (`GameplayStatics.GetGameState`)))
  (`/Game/Network_BP/MyGameState_BP.hiuhiuh` _asmy_game_state_bp))

(fn `ShootFunction`
  (params (SpawnPos :type "Transform Structure") (Location :type "Vector Structure") (Weapon :type "Actor Object Reference"))
  (`self.Shoot` SpawnPos Location Weapon))

(fn `UserConstructionScript`)