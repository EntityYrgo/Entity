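; Multiplayer GameState that keeps a match timer, tracks the player list and records kills and deaths.
; Tick uses a one-second Delay to count minutes and seconds, push them to Timer_WB widgets and call a still-empty UpdateLeaderBoard.
; UpdatePlayerList copies PlayerArray into AllPlayerStates, whose RepNotify refreshes InSession_WB widgets.
; PlayerDied updates both players' MyPlayerState_BP stats; StartGame clears all widgets, while StopGame is empty.
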(event `hiuhiuh`
  (`self.ffkyufkyu`))

(event `ffkyufkyu`
  (`KismetSystemLibrary.PrintText` "Hello"))

(event `UpdatePlayerList`
  (set `self.AllPlayerStates` (`self.PlayerArray`)))

(event `self.ReceiveTick`
  (params (DeltaSeconds :type "Float (single-precision)"))
  ;[0.5912 1 0.6312] Update LeaderBoard and Timer
  (`KismetSystemLibrary.Delay` 1.0)
  (`self.UpdateLeaderBoard`)
  (bind _result (`/Engine/EditorBlueprintResources/StandardMacros.IncrementInt` (`self.Seconds`))
    (:`  `
      (bind _output_get (set `self.Seconds` _result))
      (if (> _output_get 59)
        (bind _result_2 (`/Engine/EditorBlueprintResources/StandardMacros.IncrementInt` (`self.Minutes`))
          (:`  `
            (set `self.Minutes` _result_2)
            (set `self.Seconds` 0))))
      (bind _foundwidgets (`WidgetBlueprintLibrary.GetAllWidgetsOfClass` "/Game/Network_BP/Widgets/Timer_WB.Timer_WB_C"))
      (for _array_element _foundwidgets
        (`/Game/Network_BP/Widgets/Timer_WB.UpdateTimer` _array_element (`self.Minutes`) (`self.Seconds`))))))

(event `StartGame`
  (`WidgetLayoutLibrary.RemoveAllWidgets`))

(event `StopGame`)

(event `PlayerDied`
  (params (KilledPlayer :type "/Game/FirstPerson/Blueprints/BP_FirstPersonCharacter Object Reference") (Killer :type "/Game/FirstPerson/Blueprints/BP_FirstPersonCharacter Object Reference"))
  ;[1 0.3132 0.355] Add deaths and kills (TODO add assists)
  (bind _asmy_player_state_bp (cast `/Game/Network_BP/MyPlayerState_BP` (`Pawn.PlayerState` KilledPlayer)))
  (`/Game/Network_BP/MyPlayerState_BP.AddDeath` _asmy_player_state_bp)
  (bind _asmy_player_state_bp_2 (cast `/Game/Network_BP/MyPlayerState_BP` (`Pawn.PlayerState` Killer)))
  (`/Game/Network_BP/MyPlayerState_BP.AddKill` _asmy_player_state_bp_2))

(fn `OnRep_AllPlayerStates`
  (bind _foundwidgets (`WidgetBlueprintLibrary.GetAllWidgetsOfClass` "/Game/Network_BP/Widgets/InSession_WB.InSession_WB_C" false))
  (for _array_element _foundwidgets
    (`/Game/Network_BP/Widgets/InSession_WB.UpdateWidget` _array_element)))

(fn `UpdateLeaderBoard`)

(fn `UserConstructionScript`)