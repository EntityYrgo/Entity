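; Player state for a first-person shooter that tracks kills and deaths, relays username and spawn requests, and resolves gun and knife attacks.
; Shoot line-traces, plays the crosshair hit animation, and CheckHitBox rolls random damage by weapon class and head, body or leg box.
; Damage goes through MyGameState_BP, which also receives separate bullet effect calls for third- and first-person weapons.
; KnifeAttack deals fixed damage through its own trace.
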(event `AddKill`
  (bind _result (`/Engine/EditorBlueprintResources/StandardMacros.IncrementInt` (`self.Kills`))
    (:`  `
      (set `self.Kills` _result))))

(event `AddDeath`
  (params (Killer :type "Self Object Reference"))
  (bind _result (`/Engine/EditorBlueprintResources/StandardMacros.IncrementInt` (`self.Deaths`))
    (:`  `
      (set `self.Deaths` _result)
      (`self.AddKill` Killer))))

(event `SpawnFromPS`
  ;[0.276 0 0.214 0.417] Call spawnfunction on self
  (bind _asmy_player_controller_bp (cast `/Game/Network_BP/MyPlayerController_BP` (`self.GetPlayerController`)))
  (`/Game/Network_BP/MyPlayerController_BP.StartSpawn` _asmy_player_controller_bp))

(event `UpdateUsername`
  (params (Username :type Text))
  ;[1 0.41 0.8806] Update Username
  (bind _output_get (set `self.Username` Username))
  (bind _asmy_game_state_bp (cast `/Game/Network_BP/MyGameState_BP` (`GameplayStatics.GetGameState`)))
  (`/Game/Network_BP/MyGameState_BP.UpdateUsername_RPC` _asmy_game_state_bp self _output_get))

(event `Shoot`
  (params (StartPos :type "Vector Structure") (EndPos :type "Vector Structure") (FPWeapon :type "Actor Object Reference") (TPWeapon :type "Actor Object Reference") (Attacker :type "/Game/FirstPerson/Blueprints/BP_FirstPersonCharacter Object Reference"))
  ;[1 0.1342 0.1143] Shoot
  (set `self.EquipedWeapon` TPWeapon)
  (bind _outhit (`KismetSystemLibrary.LineTraceSingle` StartPos EndPos "TraceTypeQuery1" false (`|MakeArray` Attacker :!type "Actor Object Reference")))
  (`|ExecutionSequence`
    (:`then_0`
      (bind (_bblockinghit _binitialoverlap _time _distance _location _impactpoint _normal _impactnormal _physmat _hitactor _hitcomponent) (`GameplayStatics.BreakHitResult` _outhit))
      (bind _asbp_first_person_character (cast `/Game/FirstPerson/Blueprints/BP_FirstPersonCharacter` _hitactor))
      (bind _asbp_first_person_character_2 (cast `/Game/FirstPerson/Blueprints/BP_FirstPersonCharacter` (`self.GetPawn`)))
      (bind _crosshairwidget_ref (`/Game/FirstPerson/Blueprints/BP_FirstPersonCharacter.CrosshairWidget_Ref` _asbp_first_person_character_2))
      (`/Engine/EditorBlueprintResources/StandardMacros.IsValid` _crosshairwidget_ref
        (:`Is Valid`
          (`/Game/WidgetBlueprints/WB_Crosshair.Play Hit Animation` _crosshairwidget_ref))
        (:`Is Not Valid`
          _))
      (bind _asmy_player_state_bp (cast `/Game/Network_BP/MyPlayerState_BP` (`Pawn.PlayerState` _asbp_first_person_character)))
      (`self.CheckHitBox` _asbp_first_person_character _hitcomponent)
      (bind _asmy_game_state_bp (cast `/Game/Network_BP/MyGameState_BP` (`GameplayStatics.GetGameState`)))
      (`/Game/Network_BP/MyGameState_BP.SendDamage` _asmy_game_state_bp _asmy_player_state_bp self (`self.DamageToSend`) (`KismetMathLibrary.NegateVector` _impactnormal)))
    (:`then_1`
      (bind _asmy_game_state_bp_2 (cast `/Game/Network_BP/MyGameState_BP` (`GameplayStatics.GetGameState`)))
      (`/Game/Network_BP/MyGameState_BP.BulletFX_S` _asmy_game_state_bp_2 _outhit (`self.EquipedWeapon`) Attacker true (`self.DamageToSend`))
      (bind _output_get (set `self.EquipedWeapon` FPWeapon))
      (`/Game/Network_BP/MyGameState_BP.BulletFX_S` _asmy_game_state_bp_2 _outhit _output_get Attacker false (`self.DamageToSend`)))))

(event `KnifeAttack`
  (params (StartPos :type "Vector Structure") (EndPos :type "Vector Structure") (Attacker :type "/Game/FirstPerson/Blueprints/BP_FirstPersonCharacter Object Reference"))
  ;[0.3688 1 0.2453] Knife Attack
  (bind _outhit (`KismetSystemLibrary.LineTraceSingle` :`Start` StartPos :`End` EndPos :`TraceChannel` "TraceTypeQuery2" :`DrawDebugType` "ForDuration" :`bIgnoreSelf` false :`DrawTime` 1.0))
  (bind (_bblockinghit _binitialoverlap _time _distance _location _impactpoint _normal _impactnormal _physmat _hitactor) (`GameplayStatics.BreakHitResult` _outhit))
  (bind _asbp_first_person_character (cast `/Game/FirstPerson/Blueprints/BP_FirstPersonCharacter` _hitactor))
  (if (!= _asbp_first_person_character Attacker)
    (bind _asmy_game_state_bp (cast `/Game/Network_BP/MyGameState_BP` (`GameplayStatics.GetGameState`)))
    (bind _asmy_player_state_bp (cast `/Game/Network_BP/MyPlayerState_BP` (`Pawn.PlayerState` _asbp_first_person_character)))
    (`/Game/Network_BP/MyGameState_BP.SendDamage` _asmy_game_state_bp _asmy_player_state_bp self 75.0 (`KismetMathLibrary.NegateVector` _impactnormal))))

(fn `CheckHitBox`
  (params (PlayerActor :type "/Game/FirstPerson/Blueprints/BP_FirstPersonCharacter Object Reference") (OtherComp :type "Object Object Reference"))
  (bind _equipedweapon (`self.EquipedWeapon`))
  (`|ExecutionSequence`
    (:`then_0`
      (cast `/Game/Weapons/BP_Weapons/BP_Pistol` _equipedweapon
        (:`then`
          (set `self.HeadDamage` (`KismetMathLibrary.Conv_IntToDouble` (`KismetMathLibrary.RandomIntegerInRange` 45 53)))
          (set `self.BodyDamage` (`KismetMathLibrary.Conv_IntToDouble` (`KismetMathLibrary.RandomIntegerInRange` 8 14)))
          (set `self.LegDamage` (`KismetMathLibrary.Conv_IntToDouble` (`KismetMathLibrary.RandomIntegerInRange` 3 6))))
        (:`CastFailed`
          (cast `/Game/Weapons/BP_Weapons/BP_Rifle` _equipedweapon)
          (set `self.HeadDamage` (`KismetMathLibrary.Conv_IntToDouble` (`KismetMathLibrary.RandomIntegerInRange` 75 83)))
          (set `self.BodyDamage` (`KismetMathLibrary.Conv_IntToDouble` (`KismetMathLibrary.RandomIntegerInRange` 9 15)))
          (set `self.LegDamage` (`KismetMathLibrary.Conv_IntToDouble` (`KismetMathLibrary.RandomIntegerInRange` 4 8))))))
    (:`then_1`
      (if (== (`/Game/FirstPerson/Blueprints/BP_FirstPersonCharacter.BodyBox` PlayerActor) OtherComp)
        (set `self.DamageToSend` (`self.BodyDamage`))
        (elif (== (`/Game/FirstPerson/Blueprints/BP_FirstPersonCharacter.HeadBox` PlayerActor) OtherComp)
          (set `self.DamageToSend` (`self.HeadDamage`))
          (set `/Game/FirstPerson/Blueprints/BP_FirstPersonCharacter.IsHeadShot` true PlayerActor)
          (elif (== (`/Game/FirstPerson/Blueprints/BP_FirstPersonCharacter.LegBox` PlayerActor) OtherComp)
            (set `self.DamageToSend` (`self.LegDamage`))))))))

(fn `SpawnBulletFX`
  (params (WeaponMesh :type "MeshComponent Object Reference") (HitResult :type "HitResult Structure"))
  (bind _returnvalue (`|SpawnActorFromClass` "/Game/WeaponEffects/WeaponFX_BP.WeaponFX_BP_C" (`KismetMathLibrary.MakeTransform` (0.0 0.0 0.0)) "AlwaysSpawn" "OverrideRootScale" null WeaponMesh null))
  (`/Game/WeaponEffects/WeaponFX_BP.WeaponFire` _returnvalue HitResult (`SceneComponent.GetSocketLocation` WeaponMesh "MuzzlePos") (`SceneComponent.GetSocketLocation` WeaponMesh "ShellPos") false 0.0 null))

(fn `UserConstructionScript`)