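; Multiplayer game mode that tracks connected player controllers and their usernames, and provides player spawning.
; Login, logout and controller-swap events maintain the controller array, with login and logout also triggering a briefly delayed player-list update on the game state.
; SetUsername stores names in a controller-keyed map and copies them to the player state.
; SpawnPlayer destroys any existing pawn, then spawns and possesses a first-person character at a random PlayerStart.
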(event `self.K2_PostLogin`
  (params (NewPlayer :type "PlayerController Object Reference"))
  (bind _asmy_player_controller_bp (cast `/Game/Network_BP/MyPlayerController_BP` NewPlayer))
  (`KismetArrayLibrary.Array_Add` (`self.AllPlayerControllers`) _asmy_player_controller_bp)
  (`BlueprintMapLibrary.Map_Add` (`self.UsernameMap`) _asmy_player_controller_bp)
  (`self.UpdatePlayerList` :!label _label))

(event `self.K2_OnLogout`
  (params (ExitingController :type "Controller Object Reference"))
  (bind _asmy_player_controller_bp (cast `/Game/Network_BP/MyPlayerController_BP` ExitingController))
  (`KismetArrayLibrary.Array_RemoveItem` (`self.AllPlayerControllers`) _asmy_player_controller_bp)
  (goto _label))

(event `UpdatePlayerList`
  (`KismetSystemLibrary.Delay` 0.3)
  (bind _asmy_game_state_bp (cast `/Game/Network_BP/MyGameState_BP` (`GameplayStatics.GetGameState`)))
  (`/Game/Network_BP/MyGameState_BP.UpdatePlayerList` _asmy_game_state_bp))

(event `self.K2_OnSwapPlayerControllers`
  (params (OldPC :type "PlayerController Object Reference") (NewPC :type "PlayerController Object Reference"))
  (bind _asmy_player_controller_bp (cast `/Game/Network_BP/MyPlayerController_BP` NewPC))
  (`KismetArrayLibrary.Array_Add` (`self.AllPlayerControllers`) _asmy_player_controller_bp))

(fn `FindRandom_PlayerStart`
  (returns (PlayerStart_Transform :type "Transform Structure"))
  (bind _outactors (`GameplayStatics.GetAllActorsOfClass` "/Script/Engine.PlayerStart"))
  (return (`self.GetTransform` (`|GetArrayItem` _outactors (`KismetMathLibrary.RandomIntegerInRange` 0 (- (`KismetArrayLibrary.Array_Length` _outactors) 1))))))

(fn `GetUsername`
  (params (PlayerController :type "/Game/Network_BP/MyPlayerController_BP Object Reference"))
  (returns (Username :type Text))
  (return (`BlueprintMapLibrary.Map_Find` (`self.UsernameMap`) PlayerController)))

(fn `SetUsername`
  (params (PlayerController :type "/Game/Network_BP/MyPlayerController_BP Object Reference") (Username :type Text))
  (bind _usernamemap (`self.UsernameMap`))
  (`BlueprintMapLibrary.Map_Add` _usernamemap PlayerController Username)
  (bind _asmy_player_state_bp (cast `/Game/Network_BP/MyPlayerState_BP` (`Controller.PlayerState` PlayerController)))
  (set `/Game/Network_BP/MyPlayerState_BP.Username` (`BlueprintMapLibrary.Map_Find` _usernamemap PlayerController) _asmy_player_state_bp))

(fn `SpawnPlayer`
  (params (PlayerController :type "PlayerController Object Reference"))
  (bind _returnvalue (`Controller.K2_GetPawn` PlayerController))
  (`/Engine/EditorBlueprintResources/StandardMacros.IsValid` _returnvalue
    (:`Is Valid`
      (`self.K2_DestroyActor` _returnvalue))
    (:`Is Not Valid`
      _))
  (bind _returnvalue_2 (`|SpawnActorFromClass` "/Game/FirstPerson/Blueprints/BP_FirstPersonCharacter.BP_FirstPersonCharacter_C" (`self.FindRandom_PlayerStart`) "AdjustIfPossibleButAlwaysSpawn" "OverrideRootScale" null null))
  (`Controller.Possess` PlayerController _returnvalue_2))

(fn `UserConstructionScript`)