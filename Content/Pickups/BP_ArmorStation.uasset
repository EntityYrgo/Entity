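; Armor repair station pickup that the first-person character can detect when standing nearby.
; Its text collision overlap sets the character's PickUpOverlapping flag, then clears it and blanks the pickup text on exit.
; Getters report the name "Armor Repair", the first pickup type enumerator and zero durability/ammo.
; The repair itself is not implemented in these graphs.
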(event `self.TextCollision.OnComponentBeginOverlap`
  (params (OverlappedComponent :type "PrimitiveComponent Object Reference") (OtherActor :type "Actor Object Reference") (OtherComp :type "PrimitiveComponent Object Reference") (OtherBodyIndex :type Integer) (bFromSweep :type Boolean) (SweepResult :type "HitResult Structure (by ref)"))
  (bind _asbp_first_person_character (cast `/Game/FirstPerson/Blueprints/BP_FirstPersonCharacter` OtherActor))
  (set `/Game/FirstPerson/Blueprints/BP_FirstPersonCharacter.PickUpOverlapping` true _asbp_first_person_character))

(event `self.TextCollision.OnComponentEndOverlap`
  (params (OverlappedComponent :type "PrimitiveComponent Object Reference") (OtherActor :type "Actor Object Reference") (OtherComp :type "PrimitiveComponent Object Reference") (OtherBodyIndex :type Integer))
  (bind _asbp_first_person_character (cast `/Game/FirstPerson/Blueprints/BP_FirstPersonCharacter` OtherActor))
  (set `/Game/FirstPerson/Blueprints/BP_FirstPersonCharacter.PickUpOverlapping` false _asbp_first_person_character)
  (`/Game/WidgetBlueprints/WB_PickupText.SetText` (`/Game/FirstPerson/Blueprints/BP_FirstPersonCharacter.PickUpText_Ref` _asbp_first_person_character) ""))

(fn `GetDurability/ammo`
  (returns (`Durability/ammo` :type Integer))
  (return 0))

(fn `GetName`
  (returns (Name :type Text))
  (return "Armor Repair"))

(fn `GetPickupType`
  (returns (Pickup :type "/Game/Pickups/EPickups Enum"))
  (return "NewEnumerator0"))

(fn `UserConstructionScript`)