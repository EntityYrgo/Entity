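; Deathbox pickup actor that holds a killed player's items and exposes them through a Deathbox widget.
; On begin play it puts its widget in the viewport hidden, and CreateBox records the victim's name and fills the widget once.
; When the item count drops below zero it removes itself and restores local movement and game input; a timer also destroys it after three minutes.
; Events follow paired _S and _M relays, suggesting server-to-multicast replication.
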(event `BeginPlay_M`
  (bind _asdeathbox_wbp (cast `/Game/Pickups/Deathbox/Deathbox_WBP` (`WidgetComponent.GetUserWidgetObject` (`self.Widget`))))
  (bind _output_get (set `self.Deathbox_WidgetRef` _asdeathbox_wbp))
  (`UserWidget.AddToViewport` _output_get 0)
  (`Widget.SetVisibility` _output_get "Hidden")
  (set `/Game/Pickups/Deathbox/Deathbox_WBP.OwningBox` self (`self.Deathbox_WidgetRef`)))

(event `CreateBox_M`
  (params (DeathBoxItems :type "/Game/FirstPerson/Blueprints/DeathBoxItems Structure"))
  (set `self.Killed Player` (`.KilledPlayerName_28_6305780C49258267AFACB1AC3F490995` (break `/Game/FirstPerson/Blueprints/DeathBoxItems` DeathBoxItems)))
  (`/Engine/EditorBlueprintResources/StandardMacros.DoOnce` false
    (:`Completed`
      (`/Game/Pickups/Deathbox/Deathbox_WBP.UpdatePickups` (`self.Deathbox_WidgetRef`) DeathBoxItems))))

(event `RemoveItem_S`
  (`self.RemoveItem_M`))

(event `RemoveItem_M`
  (bind _returnvalue (`GameplayStatics.GetPlayerController` 0))
  (if (< (`/Game/Pickups/Deathbox/Deathbox_WBP.ItemsInBox` (`self.Deathbox_WidgetRef`)) 0)
    (`Widget.RemoveFromParent` (`self.Deathbox_WidgetRef`))
    (`self.RemoveBox_S`)
    (bind _asbp_first_person_character (cast `/Game/FirstPerson/Blueprints/BP_FirstPersonCharacter` (`Controller.K2_GetPawn` _returnvalue)))
    (set `/Game/FirstPerson/Blueprints/BP_FirstPersonCharacter.CanMove` true _asbp_first_person_character)
    (`WidgetBlueprintLibrary.SetInputMode_GameOnly` _returnvalue)
    (set `PlayerController.bShowMouseCursor` false _returnvalue)))

(event `self.ReceiveBeginPlay`
  (`self.BeginPlay_M`)
  (`KismetSystemLibrary.K2_SetTimerDelegate` (delegate `RemoveBox_S`) 180.0))

(event `RemoveBox_S`
  (`self.RemoveBox_M`))

(event `RemoveBox_M`
  (`self.K2_DestroyActor`))

(fn `UserConstructionScript`)