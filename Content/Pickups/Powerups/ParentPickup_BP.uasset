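; Base Blueprint for powerup pickups, which the first-person character collects by walking into them.
; On overlap it casts the other actor to BP_FirstPersonCharacter, passes its Type to that character's Pickup, then destroys itself.
; It exposes GetName, returning Name, and GetDurability/ammo, which returns zero here.
; BeginPlay only reassigns its own variables, and a direct PlayerUI update is left unconnected.
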(event `self.ReceiveBeginPlay`
  (set `self.Name` (`self.Name`))
  (set `self.Durability/ammo` (`self.Durability/ammo`)))

(event `self.ReceiveActorBeginOverlap`
  (params (OtherActor :type "Actor Object Reference"))
  (bind _asbp_first_person_character (cast `/Game/FirstPerson/Blueprints/BP_FirstPersonCharacter` OtherActor))
  (`/Game/FirstPerson/Blueprints/BP_FirstPersonCharacter.Pickup` _asbp_first_person_character (`self.type`))
  (`self.K2_DestroyActor`))

(fn `GetDurability/ammo`
  (returns (`Durability/ammo` :type Integer))
  (return 0))

(fn `GetName`
  (returns (Name :type Text))
  (return (`self.Name`)))

(fn `UserConstructionScript`)