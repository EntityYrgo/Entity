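; Kevlar powerup pickup, a child Blueprint that identifies itself to its parent pickup system.
; GetPickupType returns a fixed enum entry for this pickup's type.
; The SetMaterialColor event applies the Material variable to the Sphere component.
; Construction defers to the parent, and the BeginPlay, overlap and Tick events are disabled stubs, so this class adds no pickup logic of its own.
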(event `self.SetMaterialColor`
  (`PrimitiveComponent.SetMaterial` (`self.Sphere`) 0 (`self.Material`)))

(fn `GetPickupType`
  (returns (Pickup :type "/Game/Pickups/EPickups Enum"))
  (return "NewEnumerator7"))

(fn `UserConstructionScript`
  (`parent.UserConstructionScript`))