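; A static test enemy Blueprint that plays a death effect when a first-person projectile overlaps it.
; On BeginPlay, its skeletal mesh plays a looping forward-run animation, with no movement logic in the graph.
; An overlap with BP_FirstPersonProjectile triggers DeathEffect, which stops the animation, adds a Niagara component and hides the mesh without destroying the actor.
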(event `self.ReceiveActorBeginOverlap`
  (params (OtherActor :type "Actor Object Reference"))
  (cast `/Game/FirstPerson/Blueprints/BP_FirstPersonProjectile` OtherActor)
  (`self.DeathEffect`))

(event `self.ReceiveBeginPlay`
  (`SkeletalMeshComponent.PlayAnimation` (`self.SkeletalMesh`) "/Game/ControlRig/Characters/Mannequins/Animations/Manny/MM_Run_Fwd.MM_Run_Fwd" true))

(event `DeathEffect`
  (`SkeletalMeshComponent.Stop` (`self.SkeletalMesh`))
  (`AddComponent|NODE_AddNiagaraComponent-0`)
  (`SceneComponent.SetVisibility` (`self.SkeletalMesh`) false false))

(fn `UserConstructionScript`)