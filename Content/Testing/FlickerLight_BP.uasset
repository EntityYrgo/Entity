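; FlickerLight_BP is a test Blueprint actor whose point light flickers at random.
; Tick counts a cooldown down by delta time and fires a Flicker event roughly every tenth of a second.
; Each Flicker rolls a random float and either snaps the light to full intensity or switches it off, leaving it dark most of the time.
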(event `Flicker`
  (bind _output_get (set `self.lightFloat` (`KismetMathLibrary.RandomFloatInRange` 0.0 1.0)))
  (if (> _output_get 0.8)
    (`LightComponent.SetIntensity` (`self.PointLight`) 2500.0)
    (else
      (`LightComponent.SetIntensity` (`self.PointLight`) 0.0))))

(event `self.ReceiveTick`
  (params (DeltaSeconds :type "Float (single-precision)"))
  (bind _flickercooldown (`self.flickerCooldown`))
  (if (< _flickercooldown 0.0)
    (`self.Flicker`)
    (set `self.flickerCooldown` 0.1)
    (else
      (set `self.flickerCooldown` (- _flickercooldown DeltaSeconds)))))

(fn `UserConstructionScript`)