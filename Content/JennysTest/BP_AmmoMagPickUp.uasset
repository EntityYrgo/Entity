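; BP_AmmoMagPickUp is a pickup that grants a magazine upgrade when BP_ThirdPersonCharacter overlaps its box.
; It checks the pistol and then the rifle, requiring the weapon to be attached without a magazine already fitted.
; For an eligible weapon it raises that weapon's max ammo on the character, sets the mag-attached flag and destroys itself.
; Both checks run in one sequence, so a single pickup can upgrade both weapons.
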(event `self.Box.OnComponentBeginOverlap`
  (params (OverlappedComponent :type "PrimitiveComponent Object Reference") (OtherActor :type "Actor Object Reference") (OtherComp :type "PrimitiveComponent Object Reference") (OtherBodyIndex :type Integer) (bFromSweep :type Boolean) (SweepResult :type "HitResult Structure (by ref)"))
  (bind _player (`self.Player`))
  (bind _player_2 (`self.Player`))
  (bind _asbp_third_person_character (cast `/Game/ThirdPerson/Blueprints/BP_ThirdPersonCharacter` OtherActor))
  (bind _output_get (set `self.Player` _asbp_third_person_character))
  (`|ExecutionSequence`
    (:`then_0`
      (if (and (not (`/Game/ThirdPerson/Blueprints/BP_ThirdPersonCharacter.PistolMagAttached` (`self.Player`))) (`/Game/ThirdPerson/Blueprints/BP_ThirdPersonCharacter.PistolAttached` _output_get))
        (set `/Game/ThirdPerson/Blueprints/BP_ThirdPersonCharacter.MaxPistolAmmo` (+ (`/Game/ThirdPerson/Blueprints/BP_ThirdPersonCharacter.MaxPistolAmmo` _player) (`self.PistolMag`)) _player)
        (set `/Game/ThirdPerson/Blueprints/BP_ThirdPersonCharacter.PistolMagAttached` true (`self.Player`))
        (`self.K2_DestroyActor`)))
    (:`then_1`
      (if (and (`/Game/ThirdPerson/Blueprints/BP_ThirdPersonCharacter.RifleAttached` _output_get) (not (`/Game/ThirdPerson/Blueprints/BP_ThirdPersonCharacter.RifleMagAttached` (`self.Player`))))
        (set `/Game/ThirdPerson/Blueprints/BP_ThirdPersonCharacter.MaxRifleAmmo` (+ (`/Game/ThirdPerson/Blueprints/BP_ThirdPersonCharacter.MaxRifleAmmo` _player_2) (`self.RifleMag`)) _player_2)
        (set `/Game/ThirdPerson/Blueprints/BP_ThirdPersonCharacter.RifleMagAttached` true (`self.Player`))
        (`self.K2_DestroyActor`)))))

(fn `UserConstructionScript`)