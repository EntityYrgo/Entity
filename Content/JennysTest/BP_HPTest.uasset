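; BP_HPTest is a test actor with health and locational damage from hits on separate head, body and feet boxes.
; Health starts at MaxHealth, and each box's hit event calls ApplyDamage on itself with its own amount, highest for head, crediting AK47 as causer.
; The returned damage is subtracted from clamped Health, and reaching zero sets IsDead and destroys the actor.
; Any component hit triggers damage, with no check on what struck it.
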(event `self.ReceiveBeginPlay`
  ;[0 0 0] Event BeginPlay
  (set `self.Health` (`self.MaxHealth`)))

(event `self.HeadBox.OnComponentHit`
  (params (HitComponent :type "PrimitiveComponent Object Reference") (OtherActor :type "Actor Object Reference") (OtherComp :type "PrimitiveComponent Object Reference") (NormalImpulse :type "Vector Structure") (Hit :type "HitResult Structure (by ref)"))
  ;[0 0 0] HeadShot Damage
  (if (not (`self.isDead?`))
    (bind _returnvalue (`GameplayStatics.ApplyDamage` self 100.0 null (`self.AK_47`)))
    (bind _output_get (set `self.Health` (`KismetMathLibrary.FClamp` (- (`self.Health`) _returnvalue) 0.0 (`self.MaxHealth`))))
    (if (== _output_get 0.0)
      (set `self.isDead?` true)
      (`self.K2_DestroyActor`))))

(event `self.BodyBox.OnComponentHit`
  (params (HitComponent :type "PrimitiveComponent Object Reference") (OtherActor :type "Actor Object Reference") (OtherComp :type "PrimitiveComponent Object Reference") (NormalImpulse :type "Vector Structure") (Hit :type "HitResult Structure (by ref)"))
  ;[0 0 0] BodyShot Damage
  (if (not (`self.isDead?`))
    (bind _returnvalue (`GameplayStatics.ApplyDamage` self 35.0 null (`self.AK_47`)))
    (bind _output_get (set `self.Health` (`KismetMathLibrary.FClamp` (- (`self.Health`) _returnvalue) 0.0 (`self.MaxHealth`))))
    (if (== _output_get 0.0)
      (set `self.isDead?` true)
      (`self.K2_DestroyActor`))))

(event `self.FeetBox.OnComponentHit`
  (params (HitComponent :type "PrimitiveComponent Object Reference") (OtherActor :type "Actor Object Reference") (OtherComp :type "PrimitiveComponent Object Reference") (NormalImpulse :type "Vector Structure") (Hit :type "HitResult Structure (by ref)"))
  ;[0 0 0] FeetShot Damage
  (if (not (`self.isDead?`))
    (bind _returnvalue (`GameplayStatics.ApplyDamage` self 10.0 null (`self.AK_47`)))
    (bind _output_get (set `self.Health` (`KismetMathLibrary.FClamp` (- (`self.Health`) _returnvalue) 0.0 (`self.MaxHealth`))))
    (if (== _output_get 0.0)
      (set `self.isDead?` true)
      (`self.K2_DestroyActor`))))

(fn `UserConstructionScript`)