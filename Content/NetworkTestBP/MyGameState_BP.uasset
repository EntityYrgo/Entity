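; Game State Blueprint for a network test that shares the connected player list with the UI.
; The UpdatePlayerList event copies PlayerArray into the AllPlayerStates variable.
; Its OnRep function then finds every PlayerList_Widget and calls UpdateWidget on each, so replication of the array drives the list refresh.
; Leftover player-name lookup nodes in the event graph are never executed.
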(event `UpdatePlayerList`
  (set `self.AllPlayerStates` (`self.PlayerArray`)))

(fn `OnRep_AllPlayerStates`
  (bind _foundwidgets (`WidgetBlueprintLibrary.GetAllWidgetsOfClass` "/Game/NetworkTestBP/PlayerList_Widget.PlayerList_Widget_C" false))
  (for _array_element _foundwidgets
    (`/Game/NetworkTestBP/PlayerList_Widget.UpdateWidget` _array_element)))

(fn `UserConstructionScript`)